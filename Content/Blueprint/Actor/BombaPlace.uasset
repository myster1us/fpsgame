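; BombaPlace is a bomb site trigger that lets a ThirdPersonCharacter know it can plant a bomb.
; Entering the Box while the GameInstance's BombPlant is false sets the character's Bomb flag and Turkish "press E" message, then creates a Yazı widget on screen.
; Leaving the Box, or entering once BombPlant is true, removes that widget and clears the flag and message.
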(event OnComponentBeginOverlap(Box)
  (params (OverlappedComponent :type Primitive%20Component%20Object%20Reference) (OtherActor :type Actor%20Object%20Reference) (OtherComp :type Primitive%20Component%20Object%20Reference) (OtherBodyIndex :type Integer) (bFromSweep :type Boolean) (SweepResult :type Hit%20Result%20Structure%20%28by%20ref%29))
  (bind _asmy_game_instance (Utilities|Casting|CastToMyGameInstance (Game|GetGameInstance)))
  (if (Variables|/Game/MyGameInstance.MyGameInstance_C|GetBombPlant _asmy_game_instance)
    (bind _asthird_person_character (Utilities|Casting|CastToThirdPersonCharacter (stale OnComponentEndOverlap(Box) OtherActor)))
    (Widget|RemovefromParent (Variables|Default|GetNewVar_0))
    (Variables|/Game/ThirdPersonBP/Blueprints/ThirdPersonCharacter.ThirdPersonCharacter_C|SetMesaj _asthird_person_character "")
    (Variables|/Game/ThirdPersonBP/Blueprints/ThirdPersonCharacter.ThirdPersonCharacter_C|SetBomb? _asthird_person_character false)
    (else
      (bind _asthird_person_character_2 (Utilities|Casting|CastToThirdPersonCharacter OtherActor))
      (Variables|/Game/ThirdPersonBP/Blueprints/ThirdPersonCharacter.ThirdPersonCharacter_C|SetBomb? _asthird_person_character_2 true)
      (Variables|/Game/ThirdPersonBP/Blueprints/ThirdPersonCharacter.ThirdPersonCharacter_C|SetMesaj _asthird_person_character_2 "Bomba Kurmak İçin [E] Tuşuna Bas")
      (bind _returnvalue (UserInterface|CreateWidget "/Game/UI/Yazı.Yazı_C"))
      (Variables|Default|SetNewVar_0 _returnvalue)
      (UserInterface|Viewport|AddtoViewport _returnvalue 0))))

(event OnComponentEndOverlap(Box)
  (params (OverlappedComponent :type Primitive%20Component%20Object%20Reference) (OtherActor :type Actor%20Object%20Reference) (OtherComp :type Primitive%20Component%20Object%20Reference) (OtherBodyIndex :type Integer))
  (bind _asthird_person_character (Utilities|Casting|CastToThirdPersonCharacter OtherActor))
  (Widget|RemovefromParent (Variables|Default|GetNewVar_0))
  (Variables|/Game/ThirdPersonBP/Blueprints/ThirdPersonCharacter.ThirdPersonCharacter_C|SetMesaj _asthird_person_character "")
  (Variables|/Game/ThirdPersonBP/Blueprints/ThirdPersonCharacter.ThirdPersonCharacter_C|SetBomb? _asthird_person_character false))

(event EventBeginPlay)

(event Collision|EventActorBeginOverlap
  (params (OtherActor :type Actor%20Object%20Reference)))

(event EventTick
  (params (DeltaSeconds :type Float%20%28single-precision%29)))

(fn ConstructionScript)